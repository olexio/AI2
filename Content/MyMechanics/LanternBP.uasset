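; LanternBP is an interactive lantern actor whose point light toggles when used and notifies a linked door.
; Overlapping its capsule enables player input, and leaving disables it.
; While input is enabled, pressing E calls Acces, which toggles the light and calls LitByLantern on the referenced DoorBP on every use, whether the light turns on or off.
; Its CanUse function always returns false.
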(event OnComponentBeginOverlap(Capsule)
  (params (OverlappedComponent :type Primitive%20Component%20Object%20Reference) (OtherActor :type Actor%20Object%20Reference) (OtherComp :type Primitive%20Component%20Object%20Reference) (OtherBodyIndex :type Integer) (bFromSweep :type Boolean) (SweepResult :type Hit%20Result%20Structure%20%28by%20ref%29))
  ;[1 1 1] InputON\OFF
  (Input|EnableInput (Game|GetPlayerController 0)))

(event OnComponentEndOverlap(Capsule)
  (params (OverlappedComponent :type Primitive%20Component%20Object%20Reference) (OtherActor :type Actor%20Object%20Reference) (OtherComp :type Primitive%20Component%20Object%20Reference) (OtherBodyIndex :type Integer))
  ;[1 1 1] InputON\OFF
  (Input|DisableInput (Game|GetPlayerController 0)))

(event EventAcces
  (params (Usable :type Boolean))
  (Rendering|ToggleVisibility (Variables|Default|GetPointLight) false)
  (bind _asdoor_bp (Utilities|Casting|CastToDoorBP (Variables|Default|GetDoorBP)))
  (Default|LitbyLantern _asdoor_bp))

(event Input|KeyboardEvents|E
  (params (Key :type Key%20Structure :default "AnyKey"))
  (:Pressed
    (CallFunction|Acces false)))

(fn ConstructionScript)

(fn CanUse?
  (params (Using%20Actor :type Actor%20Object%20Reference))
  (return false))