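; DoorBP is a door the player opens and closes with the E key while inside its box trigger.
; Box overlap begin and end enable and disable input for the first player controller.
; The door only responds once a LitByLantern event marks it usable.
; A DoorRotator timeline, played or reversed according to the closed flag, drives the door mesh's world yaw.
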(event OnComponentBeginOverlap(Box)
  (params (OverlappedComponent :type Primitive%20Component%20Object%20Reference) (OtherActor :type Actor%20Object%20Reference) (OtherComp :type Primitive%20Component%20Object%20Reference) (OtherBodyIndex :type Integer) (bFromSweep :type Boolean) (SweepResult :type Hit%20Result%20Structure%20%28by%20ref%29))
  (Input|EnableInput (Game|GetPlayerController 0)))

(event OnComponentEndOverlap(Box)
  (params (OverlappedComponent :type Primitive%20Component%20Object%20Reference) (OtherActor :type Actor%20Object%20Reference) (OtherComp :type Primitive%20Component%20Object%20Reference) (OtherBodyIndex :type Integer))
  (Input|DisableInput (Game|GetPlayerController 0)))

(event Custom|DoorControls
  (if (Variables|Default|GetIsUsable?)
    (if (Variables|Default|GetIsClosed?)
      (Variables|Default|SetIsClosed? false)
      (bind _doorrot (Timeline|DoorRotator Play)
        (:Update
          (Transformation|SetWorldRotation (Variables|Default|GetSM_Door) (Math|Rotator|MakeRotator 0.0 0.0 _doorrot) false false)))
      (else
        (Variables|Default|SetIsClosed? true)
        (Timeline|DoorRotator Reverse)))))

(event Custom|LitByLantern
  (Variables|Default|SetIsUsable? true))

(event Input|KeyboardEvents|E
  (params (Key :type Key%20Structure :default "AnyKey"))
  (:Pressed
    (CallFunction|DoorControls)))

(fn ConstructionScript)